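; Turret actor Blueprint that searches for a target pawn every Tick and prints the Target's display name.
; FindBestTarget sphere-overlaps pawns within SensingRange, then runs a line-of-sight check from the Turret component on candidates, intending to pick the closest visible one.
; BestTargetLocal is never assigned in the loop, so the distance filter always passes and Target receives an empty value.
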(event `self.ReceiveTick`
  (params (DeltaSeconds :type "Float (single-precision)"))
  (`self.Find Best Target`)
  (`KismetSystemLibrary.PrintString` (`KismetSystemLibrary.GetDisplayName` (`self.Target`))))

(fn `Find Best Target`
  (locals (`BestDistance(Local)` :type "Float (double-precision)") (`CurrentDistance(Local)` :type "Float (double-precision)") (`BestTarget(Local)` :type "Actor Object Reference") (`CurrentTarget(Local)` :type "Actor Object Reference"))
  (set `local.BestDistance(Local)` (+ (`self.SensingRange`) 1.0))
  (bind _outactors (`KismetSystemLibrary.SphereOverlapActors` (`self.K2_GetActorLocation`) (`self.SensingRange`) (`|MakeArray` "ObjectTypeQuery3" :!type "EObjectTypeQuery Enum") "/Script/Engine.Actor"))
  (for _array_element _outactors
    (bind _output_get (set `local.CurrentTarget(Local)` _array_element))
    (bind _output_get_2 (set `local.CurrentDistance(Local)` (`self.GetDistanceTo` _output_get self)))
    (if (or (< _output_get_2 (`local.BestDistance(Local)`)) (not (`KismetSystemLibrary.IsValid` (`local.BestTarget(Local)`))))
      (bind _result (`/Game/Blueprints/MyFunctionsLibrary.HasLineOfSight` (`SceneComponent.K2_GetComponentLocation` (`self.Turret`)) (`self.K2_GetActorLocation` (`local.CurrentTarget(Local)`)) (`|MakeArray` self (`local.CurrentTarget(Local)`) :!type "Actor Object Reference")))
      (if _result
        (set `local.CurrentTarget(Local)` (`local.CurrentTarget(Local)`))
        (set `local.BestDistance(Local)` (`local.CurrentDistance(Local)`)))))
  (set `self.Target` (`local.BestTarget(Local)`)))

(fn `UserConstructionScript`)